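; BP_Propeller is a propeller part that spins and pushes the core object it references while active.
; Each Tick calls Spin, which rotates the mesh by a fixed per-frame step, not scaled by delta time.
; It also applies force to CoreObj's mesh at the propeller's location along its right vector, scaled by core mass and PropForce, so off-center propellers can induce torque.
; An angular-impulse spin variant remains unconnected.
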(event EventBeginPlay
  (|CallParentFunction) ; This node is disabled and will not be called.\nDrag off pins to build functionality.
)

(event Collision|EventActorBeginOverlap
  (params (OtherActor :type Actor%20Object%20Reference))
  (|CallParentFunction OtherActor) ; This node is disabled and will not be called.\nDrag off pins to build functionality.
)

(event EventTick
  (params (DeltaSeconds :type Float%20%28single-precision%29))
  (|CallParentFunction DeltaSeconds)
  (CallFunction|Spin))

(fn ConstructionScript
  (|CallParentFunction))

(fn Spin
  (bind _staticmesh (Variables|Default|GetStaticMesh))
  (bind _coreobj (Variables|Default|GetcoreObj))
  (if (Variables|Default|Getactive)
    (Transformation|AddLocalRotation (Variables|Default|GetStaticMesh) "18.000000,0.000000,0.000000" false false)
    (Class|PrimitiveComponent|AddForceatLocation (Variables|/Game/Blueprints/BP_Pickupable.BP_Pickupable_C|GetStaticMesh _coreobj) (* (* (* (Default|GetMass _coreobj) 0.1) (LocalVariables|GetpropForce)) (Math|Vector|GetRightVector _staticmesh)) (Transformation|GetWorldLocation _staticmesh) "None")))