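; BP_LevelManager starts the game's first level load and controls the loading screen.
; On BeginPlay it creates a WBP_LoadingScreen widget, adds it to the viewport, then after a short delay calls LoadLevel for the first level and spawn point.
; Tick polls the LevelLoading flag every frame to show or hide that widget.
; LoadLevel's implementation and the code that sets LevelLoading are not in these graphs.
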(event EventBeginPlay
  (bind _returnvalue (UserInterface|CreateWidget "/Game/UI/WBP_LoadingScreen.WBP_LoadingScreen_C"))
  (bind _output_get (Variables|Default|SetloadingScreen _returnvalue))
  (UserInterface|Viewport|AddtoViewport _output_get 0)
  (Utilities|FlowControl|Delay 0.2)
  (Class|LevelManager|LoadLevel))

(event EventTick
  (params (DeltaSeconds :type Float%20%28single-precision%29))
  (bind _loadingscreen (Variables|Default|GetloadingScreen))
  (if (Variables|Default|GetbLevelLoading)
    (Default|Show _loadingscreen)
    (else
      (Default|Hide _loadingscreen))))

(fn ConstructionScript)