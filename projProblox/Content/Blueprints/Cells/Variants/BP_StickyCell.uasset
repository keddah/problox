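; BP_StickyCell is a cell variant that plays a one-time hover effect when it first becomes safe.
; BeginPlay spawns FX_Hover inactive, snapped and attached to the Body component.
; Tick polls IsSafe, and on the first true result detaches the effect at its current world transform and activates it, with a flag preventing replays.
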(event EventTick
  (params (DeltaSeconds :type Float%20%28single-precision%29))
  (if (and (Class|Cell|IsSafe) (not (Variables|Default|GetfxPlayed)))
    (Variables|Default|SetfxPlayed true)
    (bind _fx (Variables|Default|Getfx)
      (:then
        (Transformation|DetachFromComponent _fx "KeepWorld" "KeepWorld" "KeepWorld" true)
        (Components|Activation|SetActive _fx true false))
      (:else))))

(event EventBeginPlay
  (bind _returnvalue (Niagara|SpawnSystemAttached "/Game/VFX/FX_Hover.FX_Hover" (Variables|Default|Getbody) "None" "0, 0, 0" "0, 0, 0" "SnapToTarget" false false))
  (Variables|Default|Setfx _returnvalue))

(fn ConstructionScript)