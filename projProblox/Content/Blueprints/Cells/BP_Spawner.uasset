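; Spawner Blueprint that fires a timed particle effect when an actor's static mesh enters its trigger.
; BeginPlay pre-spawns the inactive emitter at the VfxSpawn transform.
; Trigger overlaps skip non-mesh components such as the core's triggers, then call Overlap; on success the effect activates, runs for Duration, then stops and prints a debug message.
; The construction script counter-scales ForceDirection against the Scene component's scale.
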(event OnComponentBeginOverlap(spawnTrigger)
  (params (OverlappedComponent :type Primitive%20Component%20Object%20Reference) (OtherActor :type Actor%20Object%20Reference) (OtherComp :type Primitive%20Component%20Object%20Reference) (OtherBodyIndex :type Integer) (bFromSweep :type Boolean) (SweepResult :type Hit%20Result%20Structure%20%28by%20ref%29))
  (if (Class|GameplayStatics|ObjectIsA OtherComp "/Script/Engine.StaticMeshComponent")
    (bind _returnvalue (Class|CellSpawner|Overlap OtherActor))
    (if _returnvalue
      (bind _spawnedvfx (Variables|Default|GetspawnedVFX)
        (:then
          (Components|Activation|Activate _spawnedvfx true)
          (Utilities|FlowControl|Delay (Variables|Default|GetDuration))
          (Components|Activation|SetActive _spawnedvfx false false)
          (Development|PrintString "Hello"))
        (:else)))))

(event EventBeginPlay
  (bind _vfxspawn (Variables|Default|GetvfxSpawn))
  (bind _vfxsystem (Variables|Default|GetvfxSystem)
    (:then
      (bind _returnvalue (Effects|SpawnEmitteratLocation _vfxsystem (Transformation|GetWorldLocation _vfxspawn) (Transformation|GetWorldRotation _vfxspawn) "1.000000,1.000000,1.000000" true "None" false))
      (Variables|Default|SetspawnedVFX _returnvalue))
    (:else)))

(fn ConstructionScript
  (Transformation|SetRelativeScale3D (Variables|Default|GetforceDirection) (/ 1.0 (Variables|/Script/Engine.SceneComponent|GetRelativeScale3D (Variables|Default|Getscene)))))