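; BP_PropPropeller is a spinning propeller prop that blows physics objects along its forward axis.
; Box overlap events add components to WindContainer and remove them when they leave.
; Tick rolls the propeller by SpinSpeed, unscaled by delta time, and applies a forward force to each simulating component in the container.
; The force scales with mass plus one, so objects of different weights accelerate similarly.
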(event OnComponentBeginOverlap(Box)
  (params (OverlappedComponent :type Primitive%20Component%20Object%20Reference) (OtherActor :type Actor%20Object%20Reference) (OtherComp :type Primitive%20Component%20Object%20Reference) (OtherBodyIndex :type Integer) (bFromSweep :type Boolean) (SweepResult :type Hit%20Result%20Structure%20%28by%20ref%29))
  (Utilities|Array|AddUnique (Variables|Default|GetwindContainer) OtherComp))

(event OnComponentEndOverlap(Box)
  (params (OverlappedComponent :type Primitive%20Component%20Object%20Reference) (OtherActor :type Actor%20Object%20Reference) (OtherComp :type Primitive%20Component%20Object%20Reference) (OtherBodyIndex :type Integer))
  (Utilities|Array|RemoveItem (Variables|Default|GetwindContainer) OtherComp))

(event EventTick
  (params (DeltaSeconds :type Float%20%28single-precision%29))
  (Transformation|AddRelativeRotation (Variables|Default|Getpropeller) (Math|Rotator|MakeRotator (Variables|Default|GetspinSpeed) 0.0 0.0) false false)
  (for _array_element (Variables|Default|GetwindContainer)
    (if (Physics|IsSimulatingPhysics _array_element "None")
      (Physics|AddForce _array_element (* (Math|Vector|GetForwardVector (Variables|Default|Getpropeller)) (+ (Physics|GetMass _array_element) 1.0) (Variables|Default|Getforce) 1e+03) "None" false))))

(fn ConstructionScript)