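; BP_Gremlin is a physics-driven creature that moves toward the player's cursor location while the player is holding.
; Tick copies the cursor location from BP_Player into Goal while Holding is set, and a looping Move timer pushes Body toward Goal with a force.
; A custom velocity-dependent drag force each tick damps the motion.
; The NewLocation timer event is empty, and the random navigable-point goal logic is disconnected.
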(event Custom|NewLocation)

(event Custom|Move
  (bind _body (Variables|Default|GetBody))
  (Physics|AddForce _body (* (Math|Vector|GetUnitDirection(Vector) (Transformation|GetWorldLocation _body) (Variables|Default|Getgoal)) (Variables|Default|GetmoveSpeed)) "None" false))

(event EventBeginPlay
  (CallFunction|SetTimers)
  (bind _returnvalue (Actor|GetActorOfClass "/Game/Blueprints/BP_Player.BP_Player_C"))
  (Variables|Default|SetNewVar _returnvalue))

(event EventTick
  (params (DeltaSeconds :type Float%20%28single-precision%29))
  (bind _newvar (Variables|Default|GetNewVar))
  (CallFunction|Drag)
  (if (Variables|/Game/Blueprints/BP_Player.BP_Player_C|Getholding _newvar)
    (Variables|Default|Setgoal (.location (Default|GetCursorLocation _newvar)))))

(fn ConstructionScript)

(fn Drag
  (bind _body (Variables|Default|GetBody))
  (bind _returnvalue (Transformation|GetComponentVelocity _body))
  (Physics|AddForce _body (* (* _returnvalue (Math|Float|Sqrt (Math|Vector|VectorLength _returnvalue))) -0.8) "None" false))

(fn SetTimers
  (Utilities|Time|SetTimerbyFunctionName 0 "NewLocation" 0.5 true)
  (Utilities|Time|SetTimerbyFunctionName 0 "Move" 0.1 true))