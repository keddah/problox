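; BP_Container is a collection container that shows the share of the level's BP_Thing actors collected on a WBP_ContainerBar widget, with a minimum mark.
; BeginPlay caches the bar and player, then counts the things after a one-second delay.
; AddThing increments the collected count, updates the bar percentage and prints debug totals.
; Each Tick, FacePlayer eases the Lid's yaw toward the player while the bar widget is valid.
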(event EventBeginPlay
  (CallFunction|SetupWidget)
  (bind _returnvalue (Actor|GetActorOfClass "/Game/Blueprints/BP_PlayerCharacter.BP_PlayerCharacter_C"))
  (Variables|Default|Setplayer _returnvalue)
  (Utilities|FlowControl|Delay 1.0)
  (bind _outactors (Actor|GetAllActorsOfClass "/Game/Blueprints/BP_Thing.BP_Thing_C"))
  (Variables|Default|SetthingsInLevel (Utilities|Array|Length _outactors)))

(event EventTick
  (params (DeltaSeconds :type Float%20%28single-precision%29))
  (CallFunction|FacePlayer DeltaSeconds))

(fn ConstructionScript)

(fn AddThing
  (bind _thingsinlevel (Variables|Default|GetthingsInLevel))
  (bind _result (Math|Integer|IncrementInt (Variables|Default|GetthingCount))
    (:%20%20
      (Default|SetPercentage (Variables|Default|GetbarWidget) (/ (Math|Conversions|ToFloat(Integer) _result) (Math|Conversions|ToFloat(Integer) _thingsinlevel)))
      (Development|PrintString (Utilities|String|Append "Things in level: " (Utilities|String|ToString(Integer) _thingsinlevel)))
      (Development|PrintString (Utilities|String|Append "THings collected: " (Utilities|String|ToString(Integer) _result))))))

(fn FacePlayer
  (params (deltaTime :type Float%20%28double-precision%29))
  (bind _lid (Variables|Default|GetLid))
  (Utilities|IsValid (Variables|Default|GetbarWidget)
    (:Is%20Valid
      (Transformation|SetWorldRotation _lid (Math|Rotator|MakeRotator 0.0 0.0 (.yaw (Math|Interpolation|Ease "CircularInOut" (* deltaTime (Variables|Default|GetlookSpeed)) (Transformation|GetWorldRotation _lid) (Math|Rotator|FindLookatRotation (Transformation|GetWorldLocation _lid) (Transformation|GetActorLocation (Variables|Default|Getplayer))) true))) false false))))

(fn SetupWidget
  (bind _aswbp_container_bar (Utilities|Casting|CastToWBP_ContainerBar (UserInterface|GetWidget (Variables|Default|GetWidget))))
  (bind _output_get (Variables|Default|SetbarWidget _aswbp_container_bar))
  (Default|CalculateMinMark _output_get (Variables|Default|GetminPercentage)))