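; BP_CoreGhost is a ghost marker that shows where the cube core stood when its turn started, once the core resets.
; On BeginPlay it finds the BP_CubeCore in the level and binds to its turn-started and reset events.
; Turn start snaps the ghost to the core's transform and hides its Cube and Arrow components, while reset makes both visible again at that saved transform.
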(event Custom|Start
  (Transformation|SetActorTransform (Transformation|GetActorTransform (Variables|Default|Getcore)))
  (Development|SetHiddeninGame (Variables|Default|GetCube) true false)
  (Development|SetHiddeninGame (Variables|Default|GetArrow) true false))

(event Custom|Reset
  (Development|SetHiddeninGame (Variables|Default|GetCube) false false)
  (Development|SetHiddeninGame (Variables|Default|GetArrow) false false))

(event EventBeginPlay
  (bind _returnvalue (Actor|GetActorOfClass "/Game/Blueprints/Pickupables/Cores/BP_CubeCore.BP_CubeCore_C"))
  (bind _output_get (Variables|Default|Setcore _returnvalue))
  (Utilities|IsValid _output_get
    (:Is%20Valid
      (EventDispatchers|BindEventtoOnTurnStarted _output_get (delegate Custom|Start))
      (EventDispatchers|AssignOnReset _output_get (delegate Custom|Reset)))))

(fn ConstructionScript)