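; BP_HexCore is a pickupable core that gathers cells into a linked collector and advances waves.
; Its homer volume attracts non-safe cells, while its collector volume or added-thing event triggers CollectCell.
; CollectCell teleports the cell to the collector's collect point, increments it, and calls NextWave in Wave mode when nearly full.
; Tick permits pickup only while the core is within horizontal FairBounds distance of the collector.
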(event OnComponentBeginOverlap(thingHomer)
  (params (OverlappedComponent :type Primitive%20Component%20Object%20Reference) (OtherActor :type Actor%20Object%20Reference) (OtherComp :type Primitive%20Component%20Object%20Reference) (OtherBodyIndex :type Integer) (bFromSweep :type Boolean) (SweepResult :type Hit%20Result%20Structure%20%28by%20ref%29))
  (if (Variables|Default|GetcanCollect)
    (bind _ascell (Utilities|Casting|CastToCell OtherActor))
    (if (not (Class|Cell|IsSafe _ascell))
      (Class|Cell|SetHoming _ascell true (Variables|Default|GetthingAttraction)))
    (else
      (bind _ascell_2 (Utilities|Casting|CastToCell OtherActor))
      (Class|Cell|SetHoming _ascell_2 false 0.0))))

(event OnComponentBeginOverlap(thingCollector)
  (params (OverlappedComponent :type Primitive%20Component%20Object%20Reference) (OtherActor :type Actor%20Object%20Reference) (OtherComp :type Primitive%20Component%20Object%20Reference) (OtherBodyIndex :type Integer) (bFromSweep :type Boolean) (SweepResult :type Hit%20Result%20Structure%20%28by%20ref%29))
  (if (Variables|Default|GetcanCollect)
    (bind _ascell (Utilities|Casting|CastToCell OtherActor))
    (if (not (Class|Cell|IsSafe _ascell))
      (CallFunction|CollectCell _ascell))))

(event OnComponentEndOverlap(thingHomer)
  (params (OverlappedComponent :type Primitive%20Component%20Object%20Reference) (OtherActor :type Actor%20Object%20Reference) (OtherComp :type Primitive%20Component%20Object%20Reference) (OtherBodyIndex :type Integer))
  (bind _ascell (Utilities|Casting|CastToCell OtherActor))
  (Class|Cell|SetHoming _ascell false 0.0))

(event Custom|onAddedThing_Event
  (params (thing :type Actor%20Object%20Reference))
  ;[0 0 0] Delegate Bindings
  (bind _asbp_cell (Utilities|Casting|CastToBP_Cell thing))
  (CallFunction|CollectCell _asbp_cell))

(event Custom|DelegateBindings
  ;[0 0 0] Delegate Bindings
  (EventDispatchers|AssignOnAddedThing (delegate Custom|onAddedThing_Event)))

(event EventBeginPlay
  ;[1 0.1042 0.1042 1 32] Main Events
  (CallFunction|DelegateBindings))

(event EventTick
  (params (DeltaSeconds :type Float%20%28single-precision%29))
  (bind _returnvalue (Transformation|GetActorLocation))
  ;[1 0.1042 0.1042 1 32] Main Events
  (bind _collector (Variables|Default|Getcollector)
    (:then
      (Class|PickupableMaster|SetCanPickup (< (Math|Vector|Distance2D(Vector) (Math|Vector2D|MakeVector2D (.x (Transformation|GetActorLocation _collector)) (.y (Transformation|GetActorLocation _collector))) (Math|Vector2D|MakeVector2D (.x _returnvalue) (.y _returnvalue))) (Variables|Default|GetfairBounds))))
    (:else)))

(fn ConstructionScript
  (Transformation|SetRelativeScale3D (Variables|Default|GetobjMesh) "3.000000,3.000000,1.500000"))

(fn CollectCell
  (params (cell :type Cell%20Object%20Reference))
  (bind _asbp_collector (Utilities|Casting|CastToBP_Collector (Variables|Default|Getcollector)))
  (Utilities|IsValid _asbp_collector
    (:Is%20Valid
      (Class|Cell|Teleport cell (Class|Collector|GetCollectPoint _asbp_collector))
      (Default|CollectThing _asbp_collector)
      (bind _asbp_collector_2 (Utilities|Casting|CastToBP_Collector (Variables|Default|Getcollector)))
      (if (>= (Default|GetCurrentPercentage _asbp_collector_2) 0.975)
        (switch Utilities|FlowControl|Switch|SwitchonEGameMode (Variables|Default|GetcurrentMode)
          (:Wave
            (Class|CubeCore|NextWave)))))
    (:Is%20Not%20Valid
      (Development|PrintString "No Container Found"))))