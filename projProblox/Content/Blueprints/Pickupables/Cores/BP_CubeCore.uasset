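; BP_CubeCore is a pickupable cube core that attracts and collects cells to earn money.
; Overlap volumes home nearby cells in and collect them, sending each to the collector's depot and adding money every CellsPerMoney count.
; Level manager changes disable physics at level zero, otherwise enable it and notify attached bounce springs.
; A guarded timer respawns the core by teleporting it to the world origin.
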(event OnComponentEndOverlap(cellHomer)
  (params (OverlappedComponent :type Primitive%20Component%20Object%20Reference) (OtherActor :type Actor%20Object%20Reference) (OtherComp :type Primitive%20Component%20Object%20Reference) (OtherBodyIndex :type Integer))
  (bind _ascell (Utilities|Casting|CastToCell OtherActor))
  (Class|Cell|SetHoming _ascell false 0.0))

(event OnComponentBeginOverlap(cellCollector)
  (params (OverlappedComponent :type Primitive%20Component%20Object%20Reference) (OtherActor :type Actor%20Object%20Reference) (OtherComp :type Primitive%20Component%20Object%20Reference) (OtherBodyIndex :type Integer) (bFromSweep :type Boolean) (SweepResult :type Hit%20Result%20Structure%20%28by%20ref%29))
  (bind _ascell (Utilities|Casting|CastToCell OtherActor))
  (if (Class|Cell|UnCollected _ascell)
    (CallFunction|CollectCell _ascell)))

(event OnComponentBeginOverlap(cellHomer)
  (params (OverlappedComponent :type Primitive%20Component%20Object%20Reference) (OtherActor :type Actor%20Object%20Reference) (OtherComp :type Primitive%20Component%20Object%20Reference) (OtherBodyIndex :type Integer) (bFromSweep :type Boolean) (SweepResult :type Hit%20Result%20Structure%20%28by%20ref%29))
  (bind _ascell (Utilities|Casting|CastToCell OtherActor))
  (Class|Cell|SetHoming _ascell true (Variables|Default|GetcellAttraction)))

(event Custom|onAddedThing_Event
  (params (thing :type Actor%20Object%20Reference))
  ;[0 0 0] Delegate Bindings
  (bind _asbp_cell (Utilities|Casting|CastToBP_Cell thing))
  (CallFunction|CollectCell _asbp_cell))

(event Custom|DelegateBindings
  ;[0 0 0] Delegate Bindings
  (EventDispatchers|AssignOnAddedCell (delegate Custom|onAddedThing_Event))
  (bind _returnvalue (Actor|GetActorOfClass "/Game/Blueprints/BP_LevelManager.BP_LevelManager_C"))
  (Utilities|IsValid _returnvalue
    (:Is%20Valid
      (EventDispatchers|AssignOnLevelChanged _returnvalue (delegate Custom|changeLevel)))
    (:Is%20Not%20Valid
      (Development|PrintString "lvl manager invalid ~ core"))))

(event Custom|changeLevel
  (params (levelIndex :type Integer) (newLevel :type ELevel%20Enum :default "BuildArea"))
  (bind _mesh (Variables|Character|GetMesh))
  ;[0 0 0] Delegate Bindings
  (if (== levelIndex 0)
    (Physics|SetSimulatePhysics _mesh false)
    (else
      (Physics|SetSimulatePhysics _mesh true)
      (for _array_element (Class|CubeCore|GetCloseAttachments)
        (bind _asbp_bounce_spring (Utilities|Casting|CastToBP_BounceSpring _array_element))
        (Default|EnterLevel _asbp_bounce_spring)))))

(event EventBeginPlay
  ;[1 0.1042 0.1042 1 32] Main Events
  (CallFunction|DelegateBindings))

(fn ConstructionScript
  (Transformation|SetRelativeScale3D (Variables|Character|GetMesh) "3.000000,3.000000,3.000000")
  (Transformation|SetRelativeScale3D (Variables|Default|GetmouseDetector) "0, 0, 0"))

(fn CollectCell
  (params (cell :type Cell%20Object%20Reference))
  (bind _asbp_collector (Utilities|Casting|CastToBP_Collector (Variables|Default|Getcollector)))
  (Utilities|IsValid _asbp_collector
    (:Is%20Valid
      (Class|CubeCore|PlayCollectSound)
      (Class|Cell|ToCollector cell (Class|Collector|GetDepoPoint _asbp_collector))
      (bind _cell_count (Default|CollectThing _asbp_collector))
      (if (== (Math|Integer|%(Integer) _cell_count (Variables|Money|GetcellsPerMoney)) 0)
        (Class|CubeCore|AddMoney (Variables|Money|GetmoneyIncrements))))
    (:Is%20Not%20Valid
      (Development|PrintString "No Container Found"))))

(fn Respawn
  (bind _returnvalue (Math|Transform|MakeTransform "0, 0, 0"))
  (Class|CubeCore|Teleport (.rotation _returnvalue) (.location _returnvalue) true))

(fn BeginRespawn
  (params (respawnDelay :type Float%20%28single-precision%29))
  (if (not (Class|KismetSystemLibrary|TimerExistsHandle (Variables|Default|GetrespawnTimer)))
    (bind _returnvalue (Utilities|Time|SetTimerbyFunctionName 0 "Respawn" respawnDelay))
    (Variables|Default|SetrespawnTimer _returnvalue)))