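; BP_CubeCore is a pickupable core that attracts nearby BP_Thing actors and sends them to the level's BP_Container.
; On BeginPlay it caches the container found by GetActorOfClass as SafePlace.
; The ThingHomer overlap volume toggles homing on Things as they enter or leave.
; Things that overlap ThingCollector are teleported to the container's CollectPoint, with a debug print if no container is valid.
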(event OnComponentBeginOverlap(thingHomer)
  (params (OverlappedComponent :type Primitive%20Component%20Object%20Reference) (OtherActor :type Actor%20Object%20Reference) (OtherComp :type Primitive%20Component%20Object%20Reference) (OtherBodyIndex :type Integer) (bFromSweep :type Boolean) (SweepResult :type Hit%20Result%20Structure%20%28by%20ref%29))
  (bind _asbp_thing (Utilities|Casting|CastToBP_Thing OtherActor))
  (Class|Thing|SetHoming _asbp_thing true))

(event OnComponentBeginOverlap(thingCollector)
  (params (OverlappedComponent :type Primitive%20Component%20Object%20Reference) (OtherActor :type Actor%20Object%20Reference) (OtherComp :type Primitive%20Component%20Object%20Reference) (OtherBodyIndex :type Integer) (bFromSweep :type Boolean) (SweepResult :type Hit%20Result%20Structure%20%28by%20ref%29))
  (bind _safeplace (Variables|Default|GetsafePlace))
  (Utilities|IsValid _safeplace
    (:Is%20Valid
      (bind _asbp_thing (Utilities|Casting|CastToBP_Thing OtherActor))
      (Class|Thing|Teleport _asbp_thing (Transformation|GetWorldLocation (Variables|/Game/Blueprints/BP_Container.BP_Container_C|GetCollectPoint _safeplace))))
    (:Is%20Not%20Valid
      (Development|PrintString "No Container Found"))))

(event OnComponentEndOverlap(thingHomer)
  (params (OverlappedComponent :type Primitive%20Component%20Object%20Reference) (OtherActor :type Actor%20Object%20Reference) (OtherComp :type Primitive%20Component%20Object%20Reference) (OtherBodyIndex :type Integer))
  (bind _asbp_thing (Utilities|Casting|CastToBP_Thing OtherActor))
  (Class|Thing|SetHoming _asbp_thing false))

(event EventBeginPlay
  (bind _returnvalue (Actor|GetActorOfClass "/Game/Blueprints/BP_Container.BP_Container_C"))
  (Variables|Default|SetsafePlace _returnvalue))

(fn ConstructionScript)