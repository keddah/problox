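; Grappling hook projectile that a BP_Grappler owner launches along its launch direction, then gets pulled toward once it lands.
; On overlapping anything but itself or its owner, it stops, disables physics and collision, and attaches its mesh to the hit component.
; Each tick while attached, it calls the grappler's Pull with a normalized direction, keeping speed independent of distance.
; It destroys itself once the grappler is within the cancel distance.
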(event OnComponentBeginOverlap(collider)
  (params (OverlappedComponent :type Primitive%20Component%20Object%20Reference) (OtherActor :type Actor%20Object%20Reference) (OtherComp :type Primitive%20Component%20Object%20Reference) (OtherBodyIndex :type Integer) (bFromSweep :type Boolean) (SweepResult :type Hit%20Result%20Structure%20%28by%20ref%29))
  (bind _mesh (Variables|Character|GetMesh))
  (bind _projectilemovement (Variables|Default|GetProjectileMovement))
  (if (and (!= (Components|GetOwner) OtherActor) (!= self OtherActor))
    (Variables|/Script/Engine.MovementComponent|SetVelocity _projectilemovement "0, 0, 0")
    (Components|Activation|Deactivate _projectilemovement)
    (Physics|SetSimulatePhysics _mesh false)
    (Collision|SetCollisionEnabled _mesh "NoCollision")
    (Transformation|AttachComponentToComponent _mesh OtherComp "None" "KeepWorld" "KeepWorld" "KeepWorld" true)
    (Variables|Default|SetcanPull true)
    (Development|PrintString (Utilities|GetDisplayName OtherActor))))

(event EventTick
  (params (DeltaSeconds :type Float%20%28single-precision%29))
  (CallFunction|Pull))

(event EventBeginPlay
  (bind _asbp_grappler (Utilities|Casting|CastToBP_Grappler (Components|GetOwner)))
  (bind _output_get (Variables|Default|Setparent _asbp_grappler))
  (Variables|/Script/Engine.MovementComponent|SetVelocity (Variables|Default|GetProjectileMovement) (* (Class|Grappler|GetLaunchDir _output_get) (Variables|Default|GetlaunchForce) 1e+03)))

(fn ConstructionScript)

(fn Pull
  (bind _parent (Variables|Default|Getparent))
  (if (Variables|Default|GetcanPull)
    (bind _output_get (Variables|Default|SetshouldPull (> (Math|Vector|Distance(Vector) (Transformation|GetWorldLocation (Class|PickupableMaster|GetMesh (Variables|Default|Getparent))) (Transformation|GetWorldLocation (Variables|Character|GetMesh))) (LocalVariables|GetcancelDistance))))
    (if _output_get
      (Class|Grappler|Pull _parent (Math|Vector|Normalize (* (- (Transformation|GetWorldLocation (Class|PickupableMaster|GetMesh _parent)) (Transformation|GetWorldLocation (Variables|Character|GetMesh))) -1.0)) (* (Variables|Default|GetpullSpeed) 1e+03))
      (else
        (Variables|Default|SetcanPull false)
        (Actor|DestroyActor)))))