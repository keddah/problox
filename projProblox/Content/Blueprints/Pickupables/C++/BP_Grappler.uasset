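; BP_Grappler is a grappling-hook pickupable that fires a hook and shows a line when its ability is active.
; On Tick, an active ability spawns a BP_GrappleHook at GrappleSpawn, stores it as Hook, then immediately clears the active flag so each activation fires once.
; It then calls SetupLine and reveals GrappleLine, which Tick hides whenever it has no valid attached actor.
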(event EventBeginPlay)

(event Collision|EventActorBeginOverlap
  (params (OtherActor :type Actor%20Object%20Reference)))

(event EventTick
  (params (DeltaSeconds :type Float%20%28single-precision%29))
  (bind _grapplespawn (Variables|Default|GetgrappleSpawn))
  (bind _grappleline (Variables|Default|GetgrappleLine))
  (bind _returnvalue (Transformation|GetWorldTransform _grapplespawn))
  (Utilities|IsValid (Class|CableComponent|GetAttachedActor _grappleline)
    (:Is%20Valid
      _)
    (:Is%20Not%20Valid
      (Development|SetHiddeninGame _grappleline true false)))
  (if (Variables|Default|Getactive)
    (bind _returnvalue_2 (Game|SpawnActorfromClass "/Game/Blueprints/Pickupables/C++/BP_GrappleHook.BP_GrappleHook_C" (Math|Transform|MakeTransform (.location _returnvalue) (.rotation _returnvalue) "1.000000,1.000000,1.000000") "AlwaysSpawn" "MultiplyWithRoot" self 0))
    (Variables|Default|Sethook _returnvalue_2)
    (Class|PickupableMaster|SetAbilityActive false)
    (Class|Grappler|SetupLine)
    (Development|SetHiddeninGame (Variables|Default|GetgrappleLine) false false)))

(fn ConstructionScript)