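; Pickupable propeller part that, while active, spins its mesh and pushes the core object it belongs to.
; Each tick, Spin rotates the mesh by a fixed step and applies force to the core along the propeller's forward vector at the propeller's location.
; Force scales with the square root of core mass, so heavier builds accelerate less, and its magnitude is debug-printed.
; The construction script sets a backward placement direction.
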(event EventBeginPlay
  (|CallParentFunction) ; This node is disabled and will not be called.\nDrag off pins to build functionality.
)

(event Collision|EventActorBeginOverlap
  (params (OtherActor :type Actor%20Object%20Reference))
  (|CallParentFunction OtherActor) ; This node is disabled and will not be called.\nDrag off pins to build functionality.
)

(event EventTick
  (params (DeltaSeconds :type Float%20%28single-precision%29))
  (|CallParentFunction DeltaSeconds)
  (CallFunction|Spin))

(fn ConstructionScript
  (|CallParentFunction)
  (Variables|Default|SetplaceDirection "-1.000000,0.000000,0.000000"))

(fn Spin
  (bind _staticmesh (Variables|Default|GetStaticMesh))
  (bind _coreobj (Variables|Default|GetcoreObj))
  (bind _propforce (LocalVariables|GetpropForce))
  (bind _mass (Default|GetMass _coreobj))
  (bind _returnvalue (Math|Float|Sqrt _mass))
  (bind _returnvalue_2 (* _returnvalue _propforce))
  (if (Variables|Default|Getactive)
    (Transformation|AddLocalRotation (Variables|Default|GetStaticMesh) "0.000000,0.000000,18.000000" false false)
    (Class|PrimitiveComponent|AddForceatLocation (Variables|/Game/Blueprints/Pickupables/BP_Pickupable.BP_Pickupable_C|GetStaticMesh _coreobj) (* _returnvalue_2 (Math|Vector|GetForwardVector _staticmesh)) (Transformation|GetWorldLocation _staticmesh) "None")
    (Development|PrintString (Utilities|String|ToString(Float) _returnvalue_2))))