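; BP_BuyableObject is a buyable pickup that shows an info panel through a widget component.
; On BeginPlay it caches the WBP_BuyableInterface widget from InfoWidget, binds the show and hide events, and feeds the widget the data from GetInfo.
; Show and hide broadcasts carry a Checker object, so only the matching instance toggles its panel.
; The construction script calls UseInfoMesh.
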(event Custom|HideWidget
  (params (checker :type Buyable%20Attachment%20Object%20Reference))
  (if (== self checker)
    (Default|Hide (Variables|Default|Getwidget))))

(event Custom|ShowWidget
  (params (checker :type Buyable%20Attachment%20Object%20Reference))
  (if (== checker self)
    (Default|Show (Variables|Default|Getwidget))))

(event EventBeginPlay
  (bind _aswbp_buyable_interface (Utilities|Casting|CastToWBP_BuyableInterface (UserInterface|GetWidget (Variables|Default|GetinfoWidget))))
  (Variables|Default|Setwidget _aswbp_buyable_interface)
  (EventDispatchers|AssignOnShow (delegate Custom|ShowWidget))
  (EventDispatchers|AssignOnHide (delegate Custom|HideWidget))
  (CallFunction|SetupWidget))

(fn ConstructionScript
  (Class|BuyableAttachment|UseInfoMesh))

(fn SetupWidget
  (bind _widget (Variables|Default|Getwidget)
    (:then
      (Default|ReceiveInfo _widget (Class|BuyableAttachment|GetInfo)))
    (:else
      (Development|PrintString "couldnt setup.. bad widget ~ buyable obj"))))