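; Grapple pickupable Blueprint that drives the grapple shot visual effect from its Active flag.
; BeginPlay attaches an initially inactive FX_GrappleShot system to GrappleSpawn.
; Tick activates the effect once through a DoOnce when Active is true, and resets that gate while Active is false without explicitly deactivating the effect.
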(event EventTick
  (params (DeltaSeconds :type Float%20%28single-precision%29))
  (bind _active (Variables|Default|Getactive))
  (bind _fx (Variables|Default|Getfx)
    (:then
      (if _active
        (Utilities|FlowControl|DoOnce false :!label _label
          (:Completed
            (Components|Activation|SetActive _fx _active false))))
      (if (not _active)
        (goto _label Reset)))
    (:else)))

(event EventBeginPlay
  (bind _returnvalue (Niagara|SpawnSystemAttached "/Game/VFX/FX_GrappleShot.FX_GrappleShot" (Variables|Default|GetgrappleSpawn) "None" "0, 0, 0" "0, 0, 0" "SnapToTarget" false false))
  (bind _output_get (Variables|Default|Setfx _returnvalue))
  (Components|Activation|SetActive _output_get false false))

(fn ConstructionScript)