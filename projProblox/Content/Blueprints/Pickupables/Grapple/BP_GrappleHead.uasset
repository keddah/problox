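; BP_GrappleHead is the projectile head of a grappling hook that pulls its owning BP_Grappler toward whatever it sticks to.
; It launches along its forward vector, then on overlapping a Static or Stationary component stops, disables physics and collision, and attaches to it.
; While attached, each tick calls the grappler's Pull with a normalized direction for distance-independent speed, destroying itself once the grappler is too close or too far.
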(event OnComponentBeginOverlap(Sphere)
  (params (OverlappedComponent :type Primitive%20Component%20Object%20Reference) (OtherActor :type Actor%20Object%20Reference) (OtherComp :type Primitive%20Component%20Object%20Reference) (OtherBodyIndex :type Integer) (bFromSweep :type Boolean) (SweepResult :type Hit%20Result%20Structure%20%28by%20ref%29))
  (bind _mesh (Variables|Character|GetMesh))
  (bind _projectilemovement (Variables|Default|GetProjectileMovement))
  (switch Utilities|FlowControl|Switch|SwitchonEComponentMobility (Variables|/Script/Engine.SceneComponent|GetMobility OtherComp)
    (:Static
      _)
    (:Stationary
      _))
  (Variables|/Script/Engine.MovementComponent|SetVelocity _projectilemovement "0, 0, 0")
  (Components|Activation|Deactivate _projectilemovement)
  (Physics|SetSimulatePhysics _mesh false)
  (Collision|SetCollisionEnabled _mesh "NoCollision")
  (Transformation|AttachComponentToComponent OtherComp "None" "KeepWorld" "KeepWorld" "KeepWorld" true)
  (Variables|Pulling|SetcanPull true))

(event EventTick
  (params (DeltaSeconds :type Float%20%28single-precision%29))
  (CallFunction|Pull))

(event EventBeginPlay
  (bind _asbp_grappler (Utilities|Casting|CastToBP_Grappler (Components|GetOwner)))
  (Variables|Default|Setparent _asbp_grappler)
  (Variables|/Script/Engine.MovementComponent|SetVelocity (Variables|Default|GetProjectileMovement) (* (Transformation|GetActorForwardVector) (Variables|Default|GetlaunchForce) 1e+03)))

(fn ConstructionScript)

(fn Pull
  (bind _mesh (Variables|Character|GetMesh))
  (bind _parent (Variables|Default|Getparent))
  (bind _parent_2 (Variables|Default|Getparent))
  (bind _returnvalue (Transformation|GetWorldLocation _mesh))
  (bind _returnvalue_2 (Transformation|GetActorLocation _parent))
  (bind _returnvalue_3 (Math|Vector|Distance(Vector) _returnvalue_2 _returnvalue))
  (if (Variables|Pulling|GetcanPull)
    (if (and (> _returnvalue_3 (LocalVariables|GetcancelDistance)) (< _returnvalue_3 (LocalVariables|GetbreakDistance)))
      (Class|Grappler|Pull _parent_2 (Math|Vector|Normalize (* (- (Transformation|GetActorLocation _parent_2) (Transformation|GetWorldLocation (Variables|Character|GetMesh))) -1.0)) (* (Variables|Pulling|GetpullSpeed) 1e+03))
      (else
        (Variables|Pulling|SetcanPull false)
        (Actor|DestroyActor)))))