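; BP_GrappleHook is a projectile grapple hook that pulls its owning BP_Grappler toward whatever it hits.
; On overlap with anything except the grappler or its ObjCore, it stops, disables its physics and collision, attaches to the hit component and enables pulling.
; Each tick it sends a normalized, constant-speed pull to the grappler, destroying itself outside the cancel-to-break distance range.
; A ten-second lifespan also limits the hook.
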(event OnComponentBeginOverlap(collider)
  (params (OverlappedComponent :type Primitive%20Component%20Object%20Reference) (OtherActor :type Actor%20Object%20Reference) (OtherComp :type Primitive%20Component%20Object%20Reference) (OtherBodyIndex :type Integer) (bFromSweep :type Boolean) (SweepResult :type Hit%20Result%20Structure%20%28by%20ref%29))
  (bind _mesh (Variables|Character|GetMesh))
  (bind _parent (Variables|Default|Getparent))
  (bind _projectile (Variables|Default|Getprojectile))
  (if (and (!= _parent OtherActor) (!= OtherActor (Variables|/Script/projProblox.PickupableMaster|GetobjCore _parent)))
    (Variables|/Script/Engine.MovementComponent|SetVelocity _projectile "0, 0, 0")
    (Components|Activation|Deactivate _projectile)
    (Physics|SetSimulatePhysics _mesh false)
    (Collision|SetCollisionEnabled _mesh "NoCollision")
    (Transformation|AttachComponentToComponent _mesh OtherComp "None" "KeepWorld" "KeepWorld" "KeepWorld" true)
    (Variables|Default|SetcanPull true)))

(event EventTick
  (params (DeltaSeconds :type Float%20%28single-precision%29))
  (CallFunction|Pull))

(event EventBeginPlay
  (bind _asbp_grappler (Utilities|Casting|CastToBP_Grappler (Components|GetOwner)))
  (Variables|Default|Setparent _asbp_grappler))

(fn ConstructionScript
  (Actor|SetLifeSpan 1e+01))

(fn Pull
  (bind _mesh (Variables|Character|GetMesh))
  (bind _parent (Variables|Default|Getparent))
  (bind _parent_2 (Variables|Default|Getparent))
  (bind _returnvalue (Transformation|GetWorldLocation _mesh))
  (bind _returnvalue_2 (Class|PickupableMaster|GetMesh _parent))
  (bind _returnvalue_3 (Transformation|GetWorldLocation _returnvalue_2))
  (bind _returnvalue_4 (Math|Vector|Distance(Vector) _returnvalue_3 _returnvalue))
  (if (Variables|Default|GetcanPull)
    (if (and (> _returnvalue_4 (LocalVariables|GetcancelDistance)) (< _returnvalue_4 (LocalVariables|GetbreakDistance)))
      (Class|Grappler|Pull _parent_2 (Math|Vector|Normalize (* (- (Transformation|GetWorldLocation (Class|PickupableMaster|GetMesh _parent_2)) (Transformation|GetWorldLocation (Variables|Character|GetMesh))) -1.0)) (* (Variables|Default|GetpullSpeed) 1e+03))
      (else
        (Variables|Default|SetcanPull false)
        (Actor|DestroyActor)))))