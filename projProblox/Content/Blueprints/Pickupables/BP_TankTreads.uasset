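; BP_TankTreads is a tank tread pickupable that tracks whether it is resting on the ground.
; Its DriveTrigger overlaps add and remove Static or Stationary components in a Floors collection, ignoring Movable ones as floors.
; Grounded turns true when a floor is added and is recomputed from whether Floors is empty when overlaps end.
; The construction script sets PlaceDir to straight up.
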(event OnComponentBeginOverlap(driveTrigger)
  (params (OverlappedComponent :type Primitive%20Component%20Object%20Reference) (OtherActor :type Actor%20Object%20Reference) (OtherComp :type Primitive%20Component%20Object%20Reference) (OtherBodyIndex :type Integer) (bFromSweep :type Boolean) (SweepResult :type Hit%20Result%20Structure%20%28by%20ref%29))
  (switch Utilities|FlowControl|Switch|SwitchonEComponentMobility (Variables|/Script/Engine.SceneComponent|GetMobility OtherComp)
    (:Static
      _)
    (:Stationary
      _))
  (Variables|Default|Setgrounded true)
  (Utilities|Array|Add (Variables|Default|Getfloors) OtherComp))

(event OnComponentEndOverlap(driveTrigger)
  (params (OverlappedComponent :type Primitive%20Component%20Object%20Reference) (OtherActor :type Actor%20Object%20Reference) (OtherComp :type Primitive%20Component%20Object%20Reference) (OtherBodyIndex :type Integer))
  (bind _floors (Variables|Default|Getfloors))
  (switch Utilities|FlowControl|Switch|SwitchonEComponentMobility (Variables|/Script/Engine.SceneComponent|GetMobility OtherComp)
    (:Static
      (Utilities|Array|RemoveItem _floors OtherComp :!label _label))
    (:Stationary
      (goto _label))
    (:Movable
      _))
  (Variables|Default|Setgrounded (not (Utilities|Array|IsEmpty _floors))))

(fn ConstructionScript
  (Variables|Default|SetplaceDir "0.000000,0.000000,1.000000"))