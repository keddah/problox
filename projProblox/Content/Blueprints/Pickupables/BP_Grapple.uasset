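; BP_Grapple is a pickupable grapple ability that fires a grapple head and can drive movement on its core object.
; When Active, Ability destroys any existing head, spawns a BP_GrappleHead at the GrappleSpawn transform, sets itself as parent and clears Active.
; GetLaunchDir exposes the static mesh's up vector as the launch direction.
; Pull forwards a direction and force to CoreObj's Movement.
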(event EventTick
  (params (DeltaSeconds :type Float%20%28single-precision%29))
  (|CallParentFunction DeltaSeconds)
  (if true
    _))

(fn ConstructionScript
  (|CallParentFunction))

(fn Pull
  (params (direction :type Vector) (force :type Float%20%28double-precision%29))
  (Default|Movement (Variables|Default|GetcoreObj) direction force))

(fn GetLaunchDir
  (return (Math|Vector|GetUpVector (Variables|Default|GetStaticMesh))))

(fn Ability
  (if (Variables|Default|Getactive)
    (Utilities|IsValid (Variables|Default|GetgrappleHead)
      (:Is%20Valid
        (Actor|DestroyActor (Variables|Default|GetgrappleHead)))
      (:Is%20Not%20Valid
        _))
    (bind _returnvalue (Game|SpawnActorfromClass "/Game/Blueprints/Pickupables/BP_GrappleHead.BP_GrappleHead_C" (Transformation|GetWorldTransform (Variables|Default|GetGrappleSpawn)) "AlwaysSpawn" "MultiplyWithRoot" self 0))
    (bind _output_get (Variables|Default|SetgrappleHead _returnvalue))
    (Default|SetParent _output_get self)
    (Variables|Default|Setactive false)))