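; BP_GrappleHead is the projectile hook fired by BP_Grapple, launched along the grapple's launch direction with a ten-second lifespan.
; On overlapping anything other than its owner or the grapple's CoreObj, it stops, disables physics and attaches to the hit component.
; Each tick while attached, it has the grapple pull along a normalized direction toward the hook, then destroys itself once within CancelDistance.
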(event OnComponentBeginOverlap(Sphere)
  (params (OverlappedComponent :type Primitive%20Component%20Object%20Reference) (OtherActor :type Actor%20Object%20Reference) (OtherComp :type Primitive%20Component%20Object%20Reference) (OtherBodyIndex :type Integer) (bFromSweep :type Boolean) (SweepResult :type Hit%20Result%20Structure%20%28by%20ref%29))
  (bind _head (Variables|Default|Gethead))
  (bind _projectilemovement (Variables|Default|GetProjectileMovement))
  (if (and (!= (Components|GetOwner) OtherActor) (!= (Variables|/Game/Blueprints/Pickupables/BP_Pickupable.BP_Pickupable_C|GetcoreObj (Variables|Default|Getparent)) OtherActor))
    (Variables|/Script/Engine.MovementComponent|SetVelocity _projectilemovement "0, 0, 0")
    (Components|Activation|Deactivate _projectilemovement)
    (Physics|SetSimulatePhysics _head false)
    (Transformation|AttachComponentToComponent _head OtherComp "None" "KeepWorld" "KeepWorld" "KeepWorld" true)
    (Variables|Default|SetcanPull true)))

(event EventTick
  (params (DeltaSeconds :type Float%20%28single-precision%29))
  (CallFunction|Pull))

(event EventBeginPlay
  (bind _asbp_grapple (Utilities|Casting|CastToBP_Grapple (Components|GetOwner)))
  (bind _output_get (Variables|Default|Setparent _asbp_grapple))
  (Variables|/Script/Engine.MovementComponent|SetVelocity (Variables|Default|GetProjectileMovement) (* (Default|GetLaunchDir _output_get) (Variables|Default|GetlaunchForce) 1e+03)))

(fn ConstructionScript
  (Actor|SetLifeSpan 1e+01))

(fn SetParent
  (params (parent :type BP%20Grapple%20Object%20Reference))
  (Variables|Default|Setparent parent))

(fn Pull
  (bind _head (Variables|Default|Gethead))
  (bind _canceldistance (LocalVariables|GetcancelDistance))
  (bind _parent (Variables|Default|Getparent))
  (bind _parent_2 (Variables|Default|Getparent))
  (bind _returnvalue (Transformation|GetWorldLocation _head))
  (bind _staticmesh (Variables|/Game/Blueprints/Pickupables/BP_Pickupable.BP_Pickupable_C|GetStaticMesh _parent))
  (bind _returnvalue_2 (Transformation|GetWorldLocation _staticmesh))
  (bind _returnvalue_3 (Math|Vector|Distance(Vector) _returnvalue_2 _returnvalue))
  (bind _returnvalue_4 (> _returnvalue_3 _canceldistance))
  (if (Variables|Default|GetcanPull)
    (Development|PrintString (Utilities|String|ToString(Boolean) _returnvalue_4))
    (bind _output_get (Variables|Default|SetshouldPull _returnvalue_4))
    (if _output_get
      (Default|Pull _parent_2 (Math|Vector|Normalize (* (- (Transformation|GetWorldLocation (Variables|/Game/Blueprints/Pickupables/BP_Grapple.BP_Grapple_C|GetGrappleSpawn _parent_2)) (Transformation|GetWorldLocation (Variables|Default|Gethead))) -1.0)) (* (Variables|Default|GetpullForce) 1e+03))
      (else
        (Variables|Default|SetcanPull false)
        (Actor|DestroyActor)))))