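; BP_Piston is an attachable pickup that delivers a one-shot shove along its socket's forward axis when active and its head hits something.
; At BeginPlay it chains the collider and flat head to the object mesh.
; Hitting a physics body applies force to it and the owning core.
; Otherwise, it teleports the core mesh 250 units to clear the contact and launches it with square-root mass scaling, then deactivates.
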(event OnComponentHit(flatHead)
  (params (HitComponent :type Primitive%20Component%20Object%20Reference) (OtherActor :type Actor%20Object%20Reference) (OtherComp :type Primitive%20Component%20Object%20Reference) (NormalImpulse :type Vector :default "0, 0, 0") (Hit :type Hit%20Result%20Structure%20%28by%20ref%29))
  (bind _pushforce (Variables|Default|GetpushForce))
  (bind _objcore (Variables|Default|GetobjCore))
  (bind _objcore_2 (Variables|Default|GetobjCore))
  (bind _attachedsocket (Variables|Default|GetattachedSocket))
  (bind _flathead (Variables|Default|GetflatHead))
  (bind _returnvalue (Class|PickupableMaster|GetMesh _objcore))
  (bind _returnvalue_2 (Transformation|GetWorldLocation _flathead))
  (bind _returnvalue_3 (Class|PickupableMaster|GetMesh _objcore_2))
  (bind _returnvalue_4 (Transformation|GetSocketRotation _returnvalue _attachedsocket))
  (bind _returnvalue_5 (Math|Vector|GetForwardVector _returnvalue_4))
  (bind _returnvalue_6 (* _pushforce 1e+03 _returnvalue_5))
  (if (Variables|Default|Getactive)
    (if (Physics|IsSimulatingPhysics OtherComp "None")
      (Class|PrimitiveComponent|AddForceatLocation OtherComp (* _returnvalue_5 _pushforce 8e+04) (.ImpactPoint (Collision|BreakHitResult Hit)) "None")
      (Utilities|IsValid _objcore_2
        (:Is%20Valid
          (Class|PrimitiveComponent|AddForceatLocation _returnvalue_3 _returnvalue_6 _returnvalue_2 "None")))
      (else
        (Utilities|IsValid _objcore_2
          (:Is%20Valid
            (Transformation|AddRelativeLocation _returnvalue_3 (* _returnvalue_5 -2.5e+02) false true) ; Elevate the piston from the collision point
            (Class|PrimitiveComponent|AddForceatLocation _returnvalue_3 (* _returnvalue_6 (Math|Float|Sqrt (Class|PickupableMaster|GetMass _objcore_2)) 25.0) _returnvalue_2 "None")
            (Development|PrintString "push seldf")))))
    (Class|PickupableMaster|SetAbilityActive false)))

(event EventBeginPlay
  (bind _flathead (Variables|Default|GetflatHead))
  (Transformation|AttachComponentToComponent _flathead (Variables|Default|GetobjMesh) "None" "KeepWorld" "KeepWorld" "KeepWorld" true)
  (Transformation|AttachComponentToComponent (Variables|Default|Getcollider) _flathead "None" "KeepWorld" "KeepWorld" "KeepWorld" true))

(fn ConstructionScript
  (Variables|Default|SetplaceDir "0.000000,0.000000,-1.000000"))