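; BP_CubeCore is a pickupable cube core, scaled up in construction, that gathers BP_Thing actors into a BP_Container found at BeginPlay.
; Its ThingHomer overlap toggles homing on Things entering or leaving it.
; ThingCollector overlap teleports Things to the container's CollectPoint and calls AddThing, printing a warning if none exists.
; Every Tick it allows pickup only while the core is within FairBounds of the container.
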(event OnComponentBeginOverlap(thingHomer)
  (params (OverlappedComponent :type Primitive%20Component%20Object%20Reference) (OtherActor :type Actor%20Object%20Reference) (OtherComp :type Primitive%20Component%20Object%20Reference) (OtherBodyIndex :type Integer) (bFromSweep :type Boolean) (SweepResult :type Hit%20Result%20Structure%20%28by%20ref%29))
  (bind _asbp_thing (Utilities|Casting|CastToBP_Thing OtherActor))
  (Class|Thing|SetHoming _asbp_thing true))

(event OnComponentBeginOverlap(thingCollector)
  (params (OverlappedComponent :type Primitive%20Component%20Object%20Reference) (OtherActor :type Actor%20Object%20Reference) (OtherComp :type Primitive%20Component%20Object%20Reference) (OtherBodyIndex :type Integer) (bFromSweep :type Boolean) (SweepResult :type Hit%20Result%20Structure%20%28by%20ref%29))
  (bind _safeplace (Variables|Default|GetsafePlace))
  (Utilities|IsValid _safeplace
    (:Is%20Valid
      (bind _asbp_thing (Utilities|Casting|CastToBP_Thing OtherActor))
      (Class|Thing|Teleport _asbp_thing (Transformation|GetWorldLocation (Variables|/Game/Blueprints/BP_Container.BP_Container_C|GetCollectPoint _safeplace)))
      (Default|AddThing _safeplace))
    (:Is%20Not%20Valid
      (Development|PrintString "No Container Found"))))

(event OnComponentEndOverlap(thingHomer)
  (params (OverlappedComponent :type Primitive%20Component%20Object%20Reference) (OtherActor :type Actor%20Object%20Reference) (OtherComp :type Primitive%20Component%20Object%20Reference) (OtherBodyIndex :type Integer))
  (bind _asbp_thing (Utilities|Casting|CastToBP_Thing OtherActor))
  (Class|Thing|SetHoming _asbp_thing false))

(event EventBeginPlay
  (bind _returnvalue (Actor|GetActorOfClass "/Game/Blueprints/BP_Container.BP_Container_C"))
  (Variables|Default|SetsafePlace _returnvalue))

(event EventTick
  (params (DeltaSeconds :type Float%20%28single-precision%29))
  (bind _returnvalue (Transformation|GetActorLocation))
  (bind _safeplace (Variables|Default|GetsafePlace))
  (bind _fairbounds (Variables|Default|GetfairBounds))
  (bind _returnvalue_2 (Transformation|GetActorLocation _safeplace))
  (bind _returnvalue_3 (Math|Vector|Distance(Vector) _returnvalue_2 _returnvalue))
  (bind _returnvalue_4 (< _returnvalue_3 _fairbounds))
  (Class|PickupableMaster|SetCanPickup _returnvalue_4)
  (if _returnvalue_4
    _))

(fn ConstructionScript
  (Transformation|SetRelativeScale3D (Variables|Default|GetobjMesh) "3.000000,3.000000,3.000000"))