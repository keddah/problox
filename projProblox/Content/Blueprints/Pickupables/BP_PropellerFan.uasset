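; BP_PropellerFan is a pickupable fan that tracks the physics objects inside its WindBox volume.
; Begin overlap adds components from other actors that simulate physics to PushedObjs, and end overlap removes them.
; The construction script sets PlaceDir to negative X.
; The graphs shown only maintain the list and apply no force to it.
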(event OnComponentBeginOverlap(windBox)
  (params (OverlappedComponent :type Primitive%20Component%20Object%20Reference) (OtherActor :type Actor%20Object%20Reference) (OtherComp :type Primitive%20Component%20Object%20Reference) (OtherBodyIndex :type Integer) (bFromSweep :type Boolean) (SweepResult :type Hit%20Result%20Structure%20%28by%20ref%29))
  (if (and (!= self (Components|GetOwner OtherComp)) (Physics|IsSimulatingPhysics OtherComp "None"))
    (Utilities|Array|Add (Variables|Default|GetpushedObjs) OtherComp)))

(event OnComponentEndOverlap(windBox)
  (params (OverlappedComponent :type Primitive%20Component%20Object%20Reference) (OtherActor :type Actor%20Object%20Reference) (OtherComp :type Primitive%20Component%20Object%20Reference) (OtherBodyIndex :type Integer))
  (Utilities|Array|RemoveItem (Variables|Default|GetpushedObjs) OtherComp))

(fn ConstructionScript
  (Variables|Default|SetplaceDir "-1.000000,0.000000,0.000000"))