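; Core pickupable block that other BP_Pickupable pieces attach to, keeping track of them in an array and in per-socket connection info for six faces.
; ToggleActive flips the active state of attached pieces, and GetMass routes through CalculateMass to include attachment mass.
; SetSelected detaches it from a parent core when picked up, or socket-snaps and registers it on release.
; Placement is empty, with its socket-finding trace left disconnected.
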(event Custom|ToggleActive
  (bind _isa (Utilities|FlowControl|FlipFlop)
    (:A
      _)
    (:B
      _))
  (for _array_element (Variables|Default|GetAttachedObjects)
    (bind _asbp_pickupable (Utilities|Casting|CastToBP_Pickupable _array_element))
    (Default|SetActive _asbp_pickupable _isa)))

(event EventBeginPlay
  (|CallParentFunction) ; This node is disabled and will not be called.\nDrag off pins to build functionality.
)

(event Collision|EventActorBeginOverlap
  (params (OtherActor :type Actor%20Object%20Reference))
  (|CallParentFunction OtherActor) ; This node is disabled and will not be called.\nDrag off pins to build functionality.
)

(event EventTick
  (params (DeltaSeconds :type Float%20%28single-precision%29))
  (|CallParentFunction DeltaSeconds))

(fn ConstructionScript
  (|CallParentFunction)
  (Variables|Default|SetisCore true)
  (Variables|Default|SetcustomPivot true)
  (CallFunction|CalculateMeshCenter))

(fn CalculateMass
  (params (cubeMass :type Float%20%28double-precision%29))
  (LocalVariables|SetoverallMass cubeMass)
  (for _array_element (Variables|Default|GetAttachedObjects)
    (bind _asbp_pickupable (Utilities|Casting|CastToBP_Pickupable _array_element))
    (return (+ (CallFunction|GetMass _asbp_pickupable) (LocalVariables|GetoverallMass)))))

(fn GetMass
  (bind _mass (CallFunction|CalculateMass (|CallParentFunction)))
  (return _mass))

(fn AddAttachment
  (params (attachment :type BP%20Pickupable%20Object%20Reference))
  (Utilities|Array|AddUnique (Variables|Default|GetAttachedObjects) attachment))

(fn RemoveAttachment
  (params (attachment :type BP%20Pickupable%20Object%20Reference))
  (Utilities|Array|RemoveItem (Variables|Default|GetAttachedObjects) attachment))

(fn CalculateMeshCenter
  (|CallParentFunction)
  (Variables|Default|SetplaceRange (* (Variables|Default|GetplaceRange) (.y (Variables|/Script/Engine.SceneComponent|GetRelativeScale3D (Variables|Default|GetStaticMesh)))))
  (Transformation|SetRelativeLocation (Variables|Default|Getpivot) (Variables|Default|Getcenter) false true))

(fn Placement)

(fn SetSelected
  (params (isSelected :type Boolean))
  (bind _self self)
  (bind _coreobj (Variables|Default|GetcoreObj))
  (bind _staticmesh (Variables|Default|GetStaticMesh))
  (bind _attachedsocket (Variables|Default|GetattachedSocket))
  (bind _coreobj_2 (Variables|Default|GetcoreObj))
  (bind _coreobj_3 (Variables|Default|GetcoreObj))
  (bind _staticmesh_2 (Variables|Default|GetStaticMesh))
  (bind _coreobj_4 (Variables|Default|GetcoreObj))
  (bind _coreobj_5 (Variables|Default|GetcoreObj))
  (bind _output_get (Variables|Default|Setselected isSelected))
  (if _output_get
    (Transformation|DetachFromComponent _staticmesh "KeepWorld" "KeepWorld" "KeepWorld" true)
    (Transformation|SetActorLocation (Transformation|GetWorldLocation _staticmesh) false false)
    (Variables|Default|Setactive false)
    (Utilities|IsValid _coreobj
      (:Is%20Valid
        (CallFunction|RemoveAttachment _coreobj self)
        (switch name (Variables|Default|GetattachedSocket)
          (:Front
            (CallFunction|SetConnectionInfo _coreobj_4 0 (Utilities|Struct|MakeConnectionInfo "None" 0 false)))
          (:Back
            (CallFunction|SetConnectionInfo _coreobj_4 1 (Utilities|Struct|MakeConnectionInfo "None" 0 false)))
          (:Left
            (CallFunction|SetConnectionInfo _coreobj_4 2 (Utilities|Struct|MakeConnectionInfo "None" 0 false)))
          (:Right
            (CallFunction|SetConnectionInfo _coreobj_4 3 (Utilities|Struct|MakeConnectionInfo "None" 0 false)))
          (:Top
            (CallFunction|SetConnectionInfo _coreobj_4 4 (Utilities|Struct|MakeConnectionInfo "None" 0 false)))
          (:Down
            (CallFunction|SetConnectionInfo _coreobj_4 5 (Utilities|Struct|MakeConnectionInfo "None" 0 false))))))
    (else
      (Utilities|IsValid _coreobj_3
        (:Is%20Valid
          (CallFunction|ResetRotation false)
          (Development|PrintString (Utilities|String|ToString(Vector) (Variables|Default|GetplaceDirection)))
          (Transformation|SetWorldRotation _staticmesh_2 (Math|Rotator|MakeRotfromZ (Math|Vector|GetForwardVector (Transformation|GetSocketRotation (Variables|/Game/Blueprints/Pickupables/BP_Pickupable.BP_Pickupable_C|GetStaticMesh _coreobj_3) (Variables|Default|GetattachedSocket)))) false false)
          (Transformation|AttachComponentToComponent _staticmesh_2 (Variables|/Game/Blueprints/Pickupables/BP_Pickupable.BP_Pickupable_C|GetStaticMesh _coreobj_5) (Variables|Default|GetattachedSocket) "SnapToTarget" "KeepWorld" "KeepWorld" true)
          (CallFunction|AddAttachment _coreobj_5 self)
          (switch name _attachedsocket
            (:Front
              (CallFunction|SetConnectionInfo _coreobj_2 0 (Utilities|Struct|MakeConnectionInfo _attachedsocket _self true)))
            (:Back
              (CallFunction|SetConnectionInfo _coreobj_2 1 (Utilities|Struct|MakeConnectionInfo _attachedsocket _self true)))
            (:Left
              (CallFunction|SetConnectionInfo _coreobj_2 2 (Utilities|Struct|MakeConnectionInfo _attachedsocket _self true)))
            (:Right
              (CallFunction|SetConnectionInfo _coreobj_2 3 (Utilities|Struct|MakeConnectionInfo _attachedsocket _self true)))
            (:Top
              (CallFunction|SetConnectionInfo _coreobj_2 4 (Utilities|Struct|MakeConnectionInfo _attachedsocket _self true)))
            (:Down
              (CallFunction|SetConnectionInfo _coreobj_2 5 (Utilities|Struct|MakeConnectionInfo _attachedsocket _self true))))))))
  (Physics|SetEnableGravity (Variables|Default|GetStaticMesh) (not (Variables|Default|Getselected))))

(fn SetConnectionInfo
  (params (index :type Integer) (info :type Connection%20Info%20Structure))
  (Utilities|Array|SetArrayElem (Variables|Default|GetconnectionInfo) index info))

(fn ObjinSocket
  (params (socket :type Name))
  (bind _connectioninfo (Variables|Default|GetconnectionInfo))
  (switch name socket
    (:Front
      (return (.attached (Utilities|Array|Get(acopy) _connectioninfo))))
    (:Back
      (return (.attached (Utilities|Array|Get(acopy) _connectioninfo 1))))
    (:Left
      (return (.attached (Utilities|Array|Get(acopy) _connectioninfo 2))))
    (:Right
      (return (.attached (Utilities|Array|Get(acopy) _connectioninfo 3))))
    (:Top
      (return (.attached (Utilities|Array|Get(acopy) _connectioninfo 4))))
    (:Down
      (return (.attached (Utilities|Array|Get(acopy) _connectioninfo 5))))))