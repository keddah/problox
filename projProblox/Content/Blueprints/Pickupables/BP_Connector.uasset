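; Connector pickupable that passes its Active state to every attached object each tick and finds a socket to snap to on core objects.
; While selected, Placement line-traces from the pivot along the mesh's six local axes until it hits a BP_CoreObject.
; It stores the core mesh socket nearest the impact point as AttachedSocket, with debug trace drawing and printing; the attachment itself happens outside these graphs.
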(event EventBeginPlay
  (|CallParentFunction) ; This node is disabled and will not be called.\nDrag off pins to build functionality.
)

(event Collision|EventActorBeginOverlap
  (params (OtherActor :type Actor%20Object%20Reference))
  (|CallParentFunction OtherActor) ; This node is disabled and will not be called.\nDrag off pins to build functionality.
)

(event EventTick
  (params (DeltaSeconds :type Float%20%28single-precision%29))
  (|CallParentFunction DeltaSeconds)
  (for _array_element (Variables|Default|GetAttachedObjects)
    (Default|SetActive _array_element (Variables|Default|Getactive))))

(fn ConstructionScript
  (|CallParentFunction))

(fn Placement
  (bind _pivot (Variables|Default|Getpivot))
  (bind _returnvalue (Transformation|GetWorldLocation _pivot))
  (if (Variables|Default|Getselected)
    (bind _index (Utilities|FlowControl|ForLoopwithBreak 0 5 :!label _label)
      (:LoopBody
        (switch int _index
          (:0
            (Variables|Default|SetplaceDirection "-1.000000,0.000000,0.000000"))
          (:1
            (Variables|Default|SetplaceDirection "1.000000,0.000000,0.000000"))
          (:2
            (Variables|Default|SetplaceDirection "0.000000,-1.000000,0.000000"))
          (:3
            (Variables|Default|SetplaceDirection "-0.000000,1.000000,0.000000"))
          (:4
            (Variables|Default|SetplaceDirection "0.000000,0.000000,-1.000000"))
          (:5
            (Variables|Default|SetplaceDirection "-0.000000,0.000000,1.000000")))
        (bind _outhit (Collision|LineTraceByChannel _returnvalue (+ _returnvalue (* (Math|Vector|RotateVector (Variables|Default|GetplaceDirection) (Transformation|GetWorldRotation (Variables|Default|GetStaticMesh))) (Variables|Default|GetplaceRange))) "TraceTypeQuery1" false 0 "ForDuration" true "(R=1.000000,G=0.000000,B=0.000000,A=1.000000)" "(R=0.000000,G=1.000000,B=0.000000,A=1.000000)" 1.0))
        (if (.bBlockingHit (Collision|BreakHitResult _outhit))
          (bind _asbp_core_object (Utilities|Casting|CastToBP_CoreObject (.HitActor (Collision|BreakHitResult _outhit))))
          (bind _output_get (Variables|Default|SetcoreObj _asbp_core_object))
          (for _array_element (Transformation|GetAllSocketNames (Variables|/Game/Blueprints/Pickupables/BP_Pickupable.BP_Pickupable_C|GetStaticMesh _output_get))
            (if (< (Math|Vector|Distance(Vector) (Transformation|GetSocketLocation (Variables|/Game/Blueprints/Pickupables/BP_Pickupable.BP_Pickupable_C|GetStaticMesh _output_get) _array_element) (.ImpactPoint (Collision|BreakHitResult _outhit))) (LocalVariables|GetshortestDist))
              (LocalVariables|SetshortestDist (Math|Vector|Distance(Vector) (Transformation|GetSocketLocation (Variables|/Game/Blueprints/Pickupables/BP_Pickupable.BP_Pickupable_C|GetStaticMesh _output_get) _array_element) (.ImpactPoint (Collision|BreakHitResult _outhit))))
              (LocalVariables|SetclosestSocket _array_element)))
          (Variables|Default|SetattachedSocket (LocalVariables|GetclosestSocket))
          (goto _label Break)
          (else
            (Variables|Default|SetcoreObj 0))))
      (:Completed
        (Development|PrintString (Utilities|String|ToString(Name) (Variables|Default|GetattachedSocket)))))))