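; Pickupable object that can be moved, rotated and attached to sockets on a BP_CoreObject, with an empty per-tick Ability function.
; While selected, gravity is off and a trace along PlaceDirection tracks the closest free socket on the hit core.
; Deselecting aligns the PlaceDirection axis to that socket and attaches the mesh, while selecting detaches it.
; Core-flagged instances derive candidate socket positions at BeginPlay by averaging mesh vertices in fours.
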(event EventBeginPlay
  (CallFunction|CalculateSockets))

(event EventTick
  (params (DeltaSeconds :type Float%20%28single-precision%29))
  (CallFunction|Ability)
  (CallFunction|Placement))

(fn ConstructionScript
  (Variables|Default|SetdefaultRot (Variables|/Script/Engine.SceneComponent|GetRelativeRotation (Variables|Default|GetStaticMesh))))

(fn SetSelected
  (params (isSelected :type Boolean) (grouped :type Boolean))
  (bind _placedirection (Variables|Default|GetplaceDirection))
  (bind _attachedsocket (Variables|Default|GetattachedSocket))
  (bind _attachedsocket_2 (Variables|Default|GetattachedSocket))
  (bind _coreobj (Variables|Default|GetcoreObj))
  (bind _coreobj_2 (Variables|Default|GetcoreObj))
  (bind _staticmesh (Variables|Default|GetStaticMesh))
  (bind _staticmesh_2 (Variables|BP_Pickupable_C|GetStaticMesh _coreobj))
  (bind _returnvalue (Transformation|GetSocketRotation _staticmesh_2 _attachedsocket_2))
  (bind _returnvalue_2 (Math|Vector|GetForwardVector _returnvalue))
  (bind _output_get (Variables|Default|Setselected isSelected))
  (if _output_get
    (if (not grouped)
      _
      (else
        _))
    (Utilities|IsValid _coreobj_2
      (:Is%20Valid
        (CallFunction|RemoveAttachment _coreobj_2 (Variables|Default|GetattachedSocket))
        (Transformation|DetachFromComponent (Variables|Default|GetStaticMesh) "KeepWorld" "KeepWorld" "KeepWorld" true)
        (Variables|Default|Setactive false))
      (:Is%20Not%20Valid
        (Development|PrintString "invalid")))
    (else
      (Utilities|IsValid _coreobj
        (:Is%20Valid
          (CallFunction|ResetRotation false)
          (if (!= (.x _placedirection) 0.0)
            (Transformation|SetWorldRotation _staticmesh (Math|Rotator|MakeRotfromX _returnvalue_2) false false)
            (Transformation|AttachComponentToComponent _staticmesh _staticmesh_2 (Variables|Default|GetattachedSocket) "SnapToTarget" "KeepWorld" "KeepWorld" true :!label _label)
            (CallFunction|AddAttachment (Variables|Default|GetcoreObj) self _attachedsocket)
            (Development|PrintString (Utilities|String|Append "adding " (Utilities|String|ToString(Name) _attachedsocket)))
            (elif (!= (.y _placedirection) 0.0)
              (Transformation|SetWorldRotation _staticmesh (Math|Rotator|MakeRotfromY _returnvalue_2) false false)
              (goto _label)
              (elif (!= (.z _placedirection) 0.0)
                (Transformation|SetWorldRotation _staticmesh (Math|Rotator|MakeRotfromZ _returnvalue_2) false false)
                (goto _label)))))))))

(fn Rotate
  (params (rotation :type Rotator))
  (Transformation|AddRelativeRotation (Variables|Default|GetStaticMesh) rotation false false))

(fn ResetRotation
  (params (resetVelocity :type Boolean))
  (bind _staticmesh (Variables|Default|GetStaticMesh))
  (Transformation|SetRelativeRotation (Variables|Default|GetStaticMesh) (Variables|Default|GetdefaultRot) false false)
  (if resetVelocity
    (Class|PrimitiveComponent|SetAllPhysicsAngularVelocityinRadians _staticmesh (Math|Vector|MakeVector 0.0 0.0 0.0) false)
    (Class|PrimitiveComponent|SetAllPhysicsLinearVelocity _staticmesh "0, 0, 0" false)))

(fn Placement
  (bind _staticmesh (Variables|Default|GetStaticMesh))
  (bind _returnvalue (Transformation|GetWorldLocation _staticmesh))
  (CallFunction|GravitySelection)
  (if (Variables|Default|Getselected)
    (bind _outhit (Collision|LineTraceByChannel _returnvalue (+ _returnvalue (* (Math|Vector|RotateVector (Variables|Default|GetplaceDirection) (Transformation|GetWorldRotation _staticmesh)) (Variables|Default|GetplaceRange))) "TraceTypeQuery1" false 0 "ForDuration" true "(R=1.000000,G=0.000000,B=0.000000,A=1.000000)" "(R=0.000000,G=1.000000,B=0.000000,A=1.000000)" 1.0))
    (if (.bBlockingHit (Collision|BreakHitResult _outhit))
      (bind _asbp_core_object (Utilities|Casting|CastToBP_CoreObject (.HitActor (Collision|BreakHitResult _outhit)))
        (:then
          (bind _output_get (Variables|Default|SetcoreObj _asbp_core_object))
          (for _array_element (Transformation|GetAllSocketNames (Variables|BP_Pickupable_C|GetStaticMesh _output_get))
            (if (not (Default|ObjinSocket (Variables|Default|GetcoreObj) _array_element))
              (if (< (Math|Vector|Distance(Vector) (Transformation|GetSocketLocation (Variables|BP_Pickupable_C|GetStaticMesh _output_get) _array_element) (.ImpactPoint (Collision|BreakHitResult _outhit))) (LocalVariables|GetshortestDist))
                (LocalVariables|SetshortestDist (Math|Vector|Distance(Vector) (Transformation|GetSocketLocation (Variables|BP_Pickupable_C|GetStaticMesh _output_get) _array_element) (.ImpactPoint (Collision|BreakHitResult _outhit))))
                (LocalVariables|SetclosestSocket _array_element))))
          (Variables|Default|SetattachedSocket (LocalVariables|GetclosestSocket)))
        (:CastFailed
          (Variables|Default|SetcoreObj 0)))
      (else
        (Variables|Default|SetcoreObj 0)))))

(fn SnapRotate
  (params (zAxis :type Boolean))
  (CallFunction|Rotate (select zAxis (Math|Rotator|MakeRotator 0.0 0.0 9e+01) (Math|Rotator|MakeRotator 0.0 9e+01 0.0))))

(fn SetPosition
  (params (newPos :type Vector))
  (Transformation|SetActorLocation newPos false false))

(fn AscendDescend
  (params (moveInput :type Float%20%28double-precision%29))
  (Transformation|AddActorLocalOffset (* moveInput (Math|Vector|VectorUp)) false false))

(fn GetMass
  (return (Physics|GetMass (Variables|Default|GetStaticMesh))))

(fn SetActive
  (params (activeVal :type Boolean))
  (Variables|Default|Setactive activeVal))

(fn CalculateSockets
  (if (Variables|Default|GetisCore)
    (LocalVariables|SetposSum "0, 0, 0")
    (bind _vertices (Class|KismetProceduralMeshLibrary|GetSectionfromStaticMesh (Variables|/Script/Engine.StaticMeshComponent|GetStaticMesh (Variables|Default|GetStaticMesh))))
    (for (_array_element _array_index) _vertices
      (if (== 0 (Math|Integer|%(Integer) (+ _array_index 1) 4))
        (bind _output_get (LocalVariables|SetaveragePos (/ (LocalVariables|GetposSum) 4)))
        (LocalVariables|SetposSum "0, 0, 0")
        (Utilities|Array|AddUnique (LocalVariables|GetmeanPositions) _output_get)
        (else
          (LocalVariables|SetposSum (+ _array_element (LocalVariables|GetposSum))))))))

(fn CalculateMeshCenter
  (bind _staticmesh (Variables|Default|GetStaticMesh))
  (bind _staticmesh_2 (Variables|/Script/Engine.StaticMeshComponent|GetStaticMesh _staticmesh))
  (for _index (range 0 (- (Class|StaticMesh|GetNumSections _staticmesh_2) 1))
    (bind _vertices (Class|KismetProceduralMeshLibrary|GetSectionfromStaticMesh _staticmesh_2 0 _index))
    (for _array_element _vertices
      (LocalVariables|SetvertPos (+ _array_element (LocalVariables|GetvertPos))))
    (LocalVariables|SetvertCount (+ (Utilities|Array|Length _vertices) (LocalVariables|GetvertCount))))
  (Variables|Default|Setcenter (/ (LocalVariables|GetvertPos) (LocalVariables|GetvertCount))))

(fn GravitySelection
  (Physics|SetEnableGravity (Variables|Default|GetStaticMesh) (not (Variables|Default|Getselected))))

(fn SetCore
  (params (rCore :type BP%20Core%20Object%20Object%20Reference))
  (Variables|Default|SetcoreObj rCore))

(fn AddSocketSelection
  (params (socket :type Name))
  (Variables|Default|SetattachedSocket socket))

(fn AddAttachment
  (params (attachment :type BP%20Pickupable%20Object%20Reference) (socket :type Name))
  (Variables|Default|SetattachedSocket socket))

(fn RemoveAttachment
  (params (socket :type Name))
  (Variables|Default|SetattachedSocket "None"))

(fn Ability)