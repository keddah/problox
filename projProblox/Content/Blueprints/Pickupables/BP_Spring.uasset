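; BP_Spring is a pickupable spring whose body is a spline mesh stretched and bent between its Start and End components.
; UpdateSpline runs on construction and every tick, deriving the spline tangents and end position from both components' relative transforms, compensating for the mesh's Z scale.
; When the stored SpringHit is a blocking hit, End aligns to the impact normal to sit on the floor; otherwise it takes a fixed relative rotation.
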(event EventTick
  (params (DeltaSeconds :type Float%20%28single-precision%29))
  (CallFunction|UpdateSpline))

(fn ConstructionScript
  (CallFunction|UpdateSpline))

(fn UpdateSpline
  (bind _end (Variables|Default|Getend))
  (bind _springhit (Variables|Default|GetspringHit))
  (bind _end_2 (Variables|Default|Getend))
  (bind _returnvalue (Transformation|GetRelativeTransform _end))
  (bind (_bblockinghit _binitialoverlap _time _distance _location _impactpoint _normal _impactnormal) (Collision|BreakHitResult _springhit))
  (if _bblockinghit
    (Transformation|SetWorldRotation _end_2 (Math|Rotator|MakeRotfromZ _impactnormal) false false) ; Align with the floor
    (else
      (Transformation|SetRelativeRotation _end_2 "180.000000,0.000000,0.000000" false false)))
  (SplineMesh|SetStartandEnd (Variables|Default|GetSplineMesh) "0, 0, 0" (* (Math|Vector|GetUpVector (.rotation (Transformation|GetRelativeTransform (Variables|Default|Getstart)))) -100) (/ (+ (Math|Vector|RotateVector (.location _returnvalue) "-90.000000,0.000000,0.000000") "-100.000000,0.000000,0.000000") (.z (Variables|/Script/Engine.SceneComponent|GetRelativeScale3D (Variables|Default|GetSplineMesh)))) (* (Math|Vector|GetForwardVector (.rotation _returnvalue)) -100) true :!class /Script/Engine.SplineMeshComponent))