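; BP_Collector is a collection container that tracks gathered BP_Things against a pass percentage, shown on a WBP_ContainerBar widget.
; BeginPlay sets the bar's minimum mark and, after a short delay to allow for spawning, counts the level's Things.
; CollectThing updates the bar with the collected fraction, and getters expose current and required percentages.
; On Tick, the lid eases its yaw toward the player's view target.
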(event EventBeginPlay
  (CallFunction|SetupWidget)
  (Utilities|FlowControl|Delay 0.3) ; Since the Things are spawned after begin play...
  (bind _outactors (Actor|GetAllActorsOfClass "/Game/Blueprints/Thing/BP_Thing.BP_Thing_C"))
  (Variables|Default|SetthingsInLevel (Utilities|Array|Length _outactors)))

(event EventTick
  (params (DeltaSeconds :type Float%20%28single-precision%29))
  (CallFunction|FacePlayer DeltaSeconds))

(fn ConstructionScript)

(fn FacePlayer
  (params (deltaTime :type Float%20%28double-precision%29))
  (bind _lid (Variables|Default|GetLid))
  (Variables|Default|GetbarWidget
    (:then
      (Transformation|SetWorldRotation _lid (Math|Rotator|MakeRotator 0.0 0.0 (.yaw (Math|Interpolation|Ease "CircularInOut" (* deltaTime (Variables|Default|GetlookSpeed)) (Transformation|GetWorldRotation _lid) (Math|Rotator|FindLookatRotation (Transformation|GetWorldLocation _lid) (Transformation|GetActorLocation (Pawn|GetViewTarget (Pawn|GetController (Variables|Default|Getplayer))))) true))) false false))
    (:else)))

(fn SetupWidget
  (bind _aswbp_container_bar (Utilities|Casting|CastToWBP_ContainerBar (UserInterface|GetWidget (Variables|Default|GetWidget))))
  (bind _output_get (Variables|Default|SetbarWidget _aswbp_container_bar))
  (Default|CalculateMinMark _output_get (Variables|Default|GetminPercentage)))

(fn CollectThing
  (Class|Collector|AddThing)
  (Default|SetPercentage (Variables|Default|GetbarWidget) (/ (Math|Conversions|ToFloat(Integer) (Variables|Default|GetthingCount)) (Math|Conversions|ToFloat(Integer) (Variables|Default|GetthingsInLevel)))))

(fn GetPassPercentage
  (return (Variables|Default|GetminPercentage)))

(fn GetCurrentPercentage
  (return (Default|GetPercent (Variables|Default|GetbarWidget))))