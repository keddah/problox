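; BP_OmniCam is a camera actor that keeps itself aimed at the level's core.
; On BeginPlay it finds a cube, cuboid or hexagonal core, taking the first valid one in that order.
; Each Tick, FaceCore eases pitch and yaw toward the core by LookSpeed, blending in a randomly offset target for shake.
; AddFOV adjusts the camera's field of view within clamped limits.
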(event EventTick
  (params (DeltaSeconds :type Float%20%28single-precision%29))
  (CallFunction|FaceCore DeltaSeconds))

(event EventBeginPlay
  (bind _returnvalue (Actor|GetActorOfClass "/Game/Blueprints/Pickupables/Cores/BP_CubeCore.BP_CubeCore_C")) ; Only need the core reference so that it can be looked at
  (Utilities|IsValid _returnvalue
    (:Is%20Valid
      (Variables|Default|Setcore _returnvalue))
    (:Is%20Not%20Valid
      (bind _returnvalue_2 (Actor|GetActorOfClass "/Game/Blueprints/Pickupables/Cores/BP_CuboidCore.BP_CuboidCore_C")) ; Only need the core reference so that it can be looked at
      (Utilities|IsValid _returnvalue_2
        (:Is%20Valid
          (Variables|Default|Setcore _returnvalue_2))
        (:Is%20Not%20Valid
          (bind _returnvalue_3 (Actor|GetActorOfClass "/Game/Blueprints/Pickupables/Cores/BP_HexagonalCore.BP_HexagonalCore_C")) ; Only need the core reference so that it can be looked at
          (Utilities|IsValid _returnvalue_3
            (:Is%20Valid
              (Variables|Default|Setcore _returnvalue_3))))))))

(fn ConstructionScript)

(fn AddFOV
  (params (FOV :type Float%20%28double-precision%29))
  (bind _camera (Variables|Default|GetCamera))
  (Camera|SetFieldOfView _camera (Math|Float|Clamp(Float) (+ FOV (Variables|/Script/Engine.CameraComponent|GetFieldOfView _camera)) 3e+01 1.1e+02)))

(fn FaceCore
  (params (deltaTime :type Float%20%28double-precision%29))
  (bind _returnvalue (Transformation|GetActorLocation))
  (bind _returnvalue_2 (Math|Random|RandomUnitVector))
  (bind _returnvalue_3 (Transformation|GetActorRotation))
  (bind _core (Variables|Default|Getcore))
  (bind _lookspeed (Variables|Default|GetlookSpeed))
  (bind _shakespeed (Variables|Default|GetshakeSpeed))
  (bind _shakeintensity (Variables|Default|GetshakeIntensity))
  (bind _returnvalue_4 (Transformation|GetActorLocation _core))
  (bind _returnvalue_5 (* deltaTime _lookspeed))
  (bind _returnvalue_6 (* _returnvalue_2 _shakeintensity))
  (bind _returnvalue_7 (Math|Rotator|FindLookatRotation _returnvalue _returnvalue_4))
  (bind _returnvalue_8 (+ _returnvalue_4 _returnvalue_6))
  (bind _returnvalue_9 (Math|Rotator|FindLookatRotation _returnvalue _returnvalue_8))
  (bind _result (Math|Interpolation|Ease "CircularInOut" _shakespeed _returnvalue_7 _returnvalue_9 false))
  (bind _result_2 (Math|Interpolation|Ease "CircularInOut" _returnvalue_5 _returnvalue_3 _result true))
  (Transformation|SetActorRotation (Math|Rotator|MakeRotator 0.0 (.pitch _result_2) (.yaw _result_2))))