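; BP_CoreObject is a core object that keeps a list of attached BP_Pickupable objects, flagging itself as the core on construction.
; AddAttachment and RemoveAttachment maintain the list without duplicates, and ToggleActive uses a FlipFlop to switch the attachments' active state.
; GetMass passes the parent's mass to CalculateMass, which returns from inside its loop, so only the first attachment's mass is added.
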(event Custom|ToggleActive
  (bind _isa (Utilities|FlowControl|FlipFlop)
    (:A
      _)
    (:B
      _))
  (for _array_element (Variables|Default|GetAttachedObjects)
    (bind _asbp_pickupable (Utilities|Casting|CastToBP_Pickupable _array_element))
    (Default|SetActive _asbp_pickupable _isa)))

(event EventBeginPlay
  (|CallParentFunction) ; This node is disabled and will not be called.\nDrag off pins to build functionality.
)

(event Collision|EventActorBeginOverlap
  (params (OtherActor :type Actor%20Object%20Reference))
  (|CallParentFunction OtherActor) ; This node is disabled and will not be called.\nDrag off pins to build functionality.
)

(event EventTick
  (params (DeltaSeconds :type Float%20%28single-precision%29))
  (|CallParentFunction DeltaSeconds) ; This node is disabled and will not be called.\nDrag off pins to build functionality.
)

(fn ConstructionScript
  (|CallParentFunction)
  (Variables|Default|SetisCore true))

(fn CalculateMass
  (params (cubeMass :type Float%20%28double-precision%29))
  (LocalVariables|SetoverallMass cubeMass)
  (for _array_element (Variables|Default|GetAttachedObjects)
    (bind _asbp_pickupable (Utilities|Casting|CastToBP_Pickupable _array_element))
    (return (+ (CallFunction|GetMass _asbp_pickupable) (LocalVariables|GetoverallMass)))))

(fn GetMass
  (bind _mass (CallFunction|CalculateMass (|CallParentFunction)))
  (return _mass))

(fn AddAttachment
  (params (attachment :type BP%20Pickupable%20Object%20Reference))
  (Utilities|Array|AddUnique (Variables|Default|GetAttachedObjects) attachment))

(fn RemoveAttachment
  (params (attachment :type BP%20Pickupable%20Object%20Reference))
  (Utilities|Array|RemoveItem (Variables|Default|GetAttachedObjects) attachment))